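; BP_Spawn drives a rotating background camera view while the game instance reports that the player is in the menu.
; Each Tick it yaws its MenuCineCamera component and copies that transform onto the first actor tagged CC_Menu1.
; A DoOnce switches the first-person character to that tagged camera through ChangeCamera.
; Outside the menu it calls ChangeCamera every Tick to restore the default view, resetting the DoOnce on success.
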(event EventTick
  (params (DeltaSeconds :type Float%20%28single-precision%29))
  (if (Variables|/Game/Blueprints/GameInstance/GI_MainGameInstance.GI_MainGameInstance_C|GetisInMenu (Variables|Default|GetgiRef))
    (Transformation|AddWorldRotation (Variables|Default|GetmenuCineCamera) (Math|Rotator|MakeRotator 0.0 0.0 (Variables|Default|GetrotationRate)) false false)
    (bind _outactors (Actor|GetAllActorswithTag "CC_Menu1"))
    (Utilities|IsValid (Utilities|Array|Get(acopy) _outactors)
      (:Is%20Valid
        (Transformation|SetActorTransform (Utilities|Array|Get(acopy) _outactors) (Transformation|GetWorldTransform (Variables|Default|GetmenuCineCamera)))
        (Utilities|FlowControl|DoOnce false :!label _label
          (:Completed
            (bind _issuccessfullychanged (Default|ChangeCamera (Variables|Default|GetplayerRef) true "CC_Menu1"))
            (if _issuccessfullychanged
              (Variables|Default|SetisInCamera true)
              (else
                (Variables|Default|SetisInCamera false)
                (Development|PrintString "Failed Function: BP_Spawn -> BP_FirstPersonCharacter:Change Camera @ Tick #1" true true "(R=1.000000,G=0.000000,B=0.000000,A=1.000000)" 1e+01 "3456324"))))))
      (:Is%20Not%20Valid
        (Development|PrintString "Failed validation: BP_Spawn -> MenuCineCamera @ Tick #2" true true "(R=1.000000,G=0.000000,B=0.000000,A=1.000000)" 1e+01 "4632463426342")))
    (else
      (bind _issuccessfullychanged_2 (Default|ChangeCamera (Variables|Default|GetplayerRef) false ""))
      (if _issuccessfullychanged_2
        (Variables|Default|SetisInCamera false)
        (goto _label Reset)))))

(event EventBeginPlay
  (bind _asgi_main_game_instance (Utilities|Casting|CastToGI_MainGameInstance (Game|GetGameInstance))
    (:then
      (Variables|Default|SetgiRef _asgi_main_game_instance)
      (bind _asbp_first_person_character (Utilities|Casting|CastToBP_FirstPersonCharacter (Game|GetPlayerCharacter 0))
        (:then
          (Variables|Default|SetplayerRef _asbp_first_person_character))
        (:CastFailed
          (Development|PrintString "Failed Cast: BP_Spawn -> BP_FirstPersonCharacter @ BeginPlay #2" true true "(R=1.000000,G=0.000000,B=0.000000,A=1.000000)" 1e+01 "134513"))))
    (:CastFailed
      (Development|PrintString "Failed Cast: BP_Spawn -> GI_MainGameInstance @ BeginPlay #1" true true "(R=1.000000,G=0.000000,B=0.000000,A=1.000000)" 1e+01 "13456134"))))

(fn ConstructionScript)