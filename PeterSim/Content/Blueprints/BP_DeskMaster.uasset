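; Base Blueprint for desks that puts the first-person player into a sitting control scheme when a trace hit is reported.
; BeginPlay applies the configured actor tags and caches a reference to the BP_FirstPersonCharacter player.
; DetectTraceHitEvent forwards to DetectTraceHit, which prints a debug message and switches the player to the IMC_SittingDown mapping context, leaving the TracedChild argument unused.
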(event Custom|DetectTraceHitEvent
  (params (tracedChild :type Actor%20Object%20Reference))
  (CallFunction|DetectTraceHit tracedChild))

(event EventBeginPlay
  ;[1 1 1] BeginPlay
  (Variables|Default|SetTags (Variables|Default|GetbeginPlayTags))
  (bind _asbp_first_person_character (Utilities|Casting|CastToBP_FirstPersonCharacter (Game|GetPlayerCharacter 0)))
  (Variables|Default|SetplayerRefMaster _asbp_first_person_character))

(fn ConstructionScript)

(fn DetectTraceHit
  (params (tracedChild :type Actor%20Object%20Reference))
  (Development|PrintString "Player Sits Down" true true "(R=0.000000,G=1.000000,B=0.310021,A=1.000000)")
  ;[1 1 1] Upddate Control Scheme
  (Default|ChangeControlScheme (Variables|Default|GetplayerRefMaster) "/Game/FirstPerson/Input/IMC_SittingDown.IMC_SittingDown")
  (return))