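; Interactive desk actor with a monitor that the player can sit at and stand up from.
; An overlap trigger outlines the desk via custom depth for the player, and BeginPlay puts WBP_MonitorScreen on its widget component.
; SitPlayerDown moves the FPV_SitDown-tagged cine camera to the monitor, teleports the player to the seat and toggles the HUD monitor screen.
; IA_StandUp restores walking controls and the default camera, toggling the screen again.
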(event OnComponentBeginOverlap(HighlightTriggerArea)
  (params (OverlappedComponent :type Primitive%20Component%20Object%20Reference) (OtherActor :type Actor%20Object%20Reference) (OtherComp :type Primitive%20Component%20Object%20Reference) (OtherBodyIndex :type Integer) (bFromSweep :type Boolean) (SweepResult :type Hit%20Result%20Structure%20%28by%20ref%29))
  ;[1 1 1] Look for Highlight
  (if (Actor|ActorHasTag OtherActor "Player")
    (Development|PrintString "hasTag" true true "(R=0.000000,G=0.660000,B=1.000000,A=1.000000)" 2.0 "deskHighlight")
    (Rendering|SetRenderCustomDepth (Variables|Default|GetDeskMesh) true)
    (Development|PrintString "On" true true "(R=0.000000,G=0.660000,B=1.000000,A=1.000000)" 2.0 "deskHighlight")
    (else
      (Development|PrintString "hasNotTag" true true "(R=0.000000,G=0.660000,B=1.000000,A=1.000000)" 2.0 "deskHighlight"))))

(event OnComponentEndOverlap(HighlightTriggerArea)
  (params (OverlappedComponent :type Primitive%20Component%20Object%20Reference) (OtherActor :type Actor%20Object%20Reference) (OtherComp :type Primitive%20Component%20Object%20Reference) (OtherBodyIndex :type Integer))
  ;[1 1 1] Look for Highlight
  (Development|PrintString "Exit" true true "(R=0.000000,G=0.660000,B=1.000000,A=1.000000)" 2.0 "deskHighlight")
  (Rendering|SetRenderCustomDepth (Variables|Default|GetDeskMesh) false)
  (Development|PrintString "Off" true true "(R=0.000000,G=0.660000,B=1.000000,A=1.000000)" 2.0 "deskHighlight"))

(event Input|EnhancedActionEvents|EnhancedInputActionIA_StandUp
  (params (ActionValue :type Boolean) (ElapsedSeconds :type Float%20%28double-precision%29) (TriggeredSeconds :type Float%20%28double-precision%29) (InputAction :type Input%20Action%20Object%20Reference :default "/Game/FirstPerson/Input/Actions/IA_StandUp.IA_StandUp"))
  (:Started
    (Development|PrintString "Hallo!")
    (CallFunction|StandPlayerUp))
  (:Completed
    (Development|PrintString "America Ya! :D")))

(event EventTick
  (params (DeltaSeconds :type Float%20%28single-precision%29))
  (Development|PrintString (Utilities|String|ToString(Transform) (Transformation|GetWorldTransform (Variables|Default|GetMonitorCameraPosition))) true true "(R=0.000000,G=1.000000,B=0.605614,A=1.000000)" 2.0 "Damian"))

(event EventBeginPlay
  (bind _asbp_first_person_character (Utilities|Casting|CastToBP_FirstPersonCharacter (Game|GetPlayerCharacter 0)))
  (Variables|Default|SetplayerRefMaster _asbp_first_person_character)
  (Variables|Default|SetTags (Variables|Default|GetbeginPlayTags))
  (Input|EnableInput (Game|GetPlayerController 0))
  (bind _returnvalue (UserInterface|CreateWidget "/Game/UserInterface/WBP_MonitorScreen.WBP_MonitorScreen_C" (Game|GetPlayerController 0)))
  (bind _output_get (Variables|Default|SetWBP_MonitorWidget _returnvalue))
  (UserInterface|SetWidget (Variables|Default|GetMonitorScreenWidget) _output_get))

(fn ConstructionScript
  (|CallParentFunction))

(fn SitPlayerDown
  (bind _playerrefmaster (Variables|Default|GetplayerRefMaster))
  (CallFunction|GetCameratoPosition)
  ;[1 1 1] Teleport player to seat
  (Transformation|SetActorLocation (Variables|Default|GetplayerRefMaster) (Transformation|GetWorldLocation (Variables|Default|GetPlayerAttachement)) false true)
  ;[1 1 1] change cursor and input mode
  (bind _action_output (Default|UpdateCursor _playerrefmaster false false false true))
  (Development|PrintString _action_output)
  ;[1 1 1] Turn screen on
  (bind _aswbp_hud (Utilities|Casting|CastToWBP_HUD (Variables|/Game/FirstPerson/Blueprints/BP_FirstPersonCharacter.BP_FirstPersonCharacter_C|Gethud_Ref _playerrefmaster)))
  (bind _isvisible (Default|ToggleMonitorScreen _aswbp_hud))
  (if _isvisible
    (return true)
    (else
      (return false))))

(fn StandPlayerUp
  (bind _playerrefmaster (Variables|Default|GetplayerRefMaster))
  ;[1 1 1] Update Control Scheme
  (Default|ChangeControlScheme (Variables|Default|GetplayerRefMaster) "/Game/FirstPerson/Input/IMC_Walking.IMC_Walking")
  ;[1 1 1] change cursor and input mode
  (bind _action_output (Default|UpdateCursor (Variables|Default|GetplayerRefMaster) false false false true))
  (Development|PrintString _action_output)
  (Default|ChangeCamera _playerrefmaster false "None")
  (bind _aswbp_hud (Utilities|Casting|CastToWBP_HUD (Variables|/Game/FirstPerson/Blueprints/BP_FirstPersonCharacter.BP_FirstPersonCharacter_C|Gethud_Ref _playerrefmaster)))
  (bind _isvisible (Default|ToggleMonitorScreen _aswbp_hud))
  (if _isvisible
    (Development|PrintString "motherfucking failed standing up" true true "(R=1.000000,G=0.000000,B=0.243276,A=1.000000)" 1e+01)
    (return false)
    (else
      (Development|PrintString "mofo stood up" true true "(R=0.000000,G=1.000000,B=0.007329,A=1.000000)" 1e+01)
      (return true))))

(fn GetCameratoPosition
  (bind _outactors (Actor|GetAllActorsOfClass "/Script/CinematicCamera.CineCameraActor"))
  (bind _array_element (Utilities|Array|ForEachLoopwithBreak _outactors :!label _label)
    (:LoopBody
      (if (Actor|ActorHasTag _array_element "FPV_SitDown")
        (goto _label Break)))
    (:Completed
      (Transformation|SetWorldTransform (Variables|/Script/Engine.Actor|GetRootComponent _array_element) (Transformation|GetWorldTransform (Variables|Default|GetMonitorCameraPosition)) false true))))