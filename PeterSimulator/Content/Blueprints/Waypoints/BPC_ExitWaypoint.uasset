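; Waypoint Blueprint that marks an exit, extending a parent waypoint class.
; On BeginPlay it adds the "Exit" tag to BeginPlayTags before calling the parent's BeginPlay, then sets ExitType to "Main".
; It finishes with a long-lived, keyed debug print naming the exit type and the waypoint's display name.
; The construction script only calls the parent.
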(event EventBeginPlay
  ;[1 1 1] Adds reception tags
  (Utilities|Array|Add (Variables|Default|GetBeginPlayTags) "Exit")
  (|CallParentFunction)
  (Variables|Default|SetexitType "Main")
  (Development|PrintString (Utilities|String|ToString(Text) (Utilities|Text|FormatText "This is a {type} exit from {waypoint display} waypoint" (Variables|Default|GetexitType) (Utilities|GetDisplayName self))) true true "(R=0.840997,G=1.000000,B=0.916238,A=1.000000)" 6e+01 "534867354"))

(fn ConstructionScript
  (|CallParentFunction))