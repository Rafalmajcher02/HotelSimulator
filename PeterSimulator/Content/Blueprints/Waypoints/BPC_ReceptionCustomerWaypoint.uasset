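; Waypoint Blueprint for reception customers, marking a queue point with a capped line length.
; On BeginPlay it adds the ReceptionCustomer tag to BeginPlayTags before calling the parent BeginPlay, then sets its queue limit.
; It prints an on-screen debug message with the waypoint name, queue limit and current queue.
; The construction script only calls the parent.
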(event EventBeginPlay
  ;[1 1 1] Adds reception tags
  (Utilities|Array|Add (Variables|Default|GetBeginPlayTags) "ReceptionCustomer")
  (|CallParentFunction)
  (Variables|Default|SetQueueLimit 10)
  (Development|PrintString (Utilities|String|ToString(Text) (Utilities|Text|FormatText "I'm waypoint {waypoint} with maximum queue of {maxQu} and current queue of {cQ}" (Utilities|GetObjectName self) (Variables|Default|GetQueueLimit) (Variables|Default|GetCurrentQueue))) true true "(R=0.840997,G=1.000000,B=0.916238,A=1.000000)" 6e+01 "3242342353463546"))

(fn ConstructionScript
  (|CallParentFunction))