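; Interactable reception desk with a monitor screen widget, which highlights through custom depth on focus and seats the first-person player.
; Interacting flips InteractToggle via InteractOnServer; its RepNotify calls SitPlayerDown whatever the value.
; Sitting moves the FPV_SitDown-tagged cine camera to the monitor, teleports the player, swaps input mapping and toggles the HUD monitor screen.
; StandPlayerUp restores camera and walking controls but is not called here.
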(event Custom|InteractOnServer
  (Variables|Default|SetInteractToggle (not (Variables|Default|GetInteractToggle)))
  (Development|PrintString "toggled"))

(event EventTick
  (params (DeltaSeconds :type Float%20%28single-precision%29))
  (Development|PrintString (Utilities|String|ToString(Transform) (Transformation|GetWorldTransform (Variables|Default|GetMonitorCameraPosition))) true true "(R=0.000000,G=1.000000,B=0.605614,A=1.000000)" 2.0 "Damian"))

(event EventBeginPlay
  (bind _asbp_first_person_character (Utilities|Casting|CastToBP_FirstPersonCharacter (Game|GetPlayerCharacter 0)))
  (bind _output_get (Variables|Default|SetplayerRefMaster _asbp_first_person_character))
  (Variables|/Game/FirstPerson/Blueprints/BP_FirstPersonCharacter.BP_FirstPersonCharacter_C|SetreceptionDeskReference _output_get self)
  (Variables|Default|SetTags (Variables|Default|GetbeginPlayTags))
  (Input|EnableInput (Game|GetPlayerController 0))
  (bind _returnvalue (UserInterface|CreateWidget "/Game/UserInterface/WBP_MonitorScreen.WBP_MonitorScreen_C" (Game|GetPlayerController 0)))
  (bind _output_get_2 (Variables|Default|SetWBP_MonitorWidget _returnvalue))
  (UserInterface|SetWidget (Variables|Default|GetMonitorScreenWidget) _output_get_2))

(event EventInterfaceToggleFocus
  (params (Focus :type Boolean))
  (Development|PrintString (Utilities|String|ToString(Boolean) Focus) true true "(R=1.000000,G=0.000000,B=0.148264,A=1.000000)" 5.0 "654365346")
  (Rendering|SetRenderCustomDepth (Variables|Default|GetDeskMesh) Focus))

(event EventInterfaceInteract
  (CallFunction|InteractonServer))

(fn ConstructionScript
  (|CallParentFunction))

(fn SitPlayerDown
  (bind _playerrefmaster (Variables|Default|GetplayerRefMaster))
  (CallFunction|GetCameratoPosition)
  ;[1 1 1] Teleport player to seat
  (Transformation|SetActorLocation (Variables|Default|GetplayerRefMaster) (Transformation|GetWorldLocation (Variables|Default|GetPlayerAttachement)) false true)
  (Default|ChangeControlScheme _playerrefmaster "/Game/FirstPerson/Input/IMC_SittingDown.IMC_SittingDown")
  ;[1 1 1] change cursor and input mode
  (bind _action_output (Default|UpdateCursor _playerrefmaster true false false true))
  (Development|PrintString _action_output)
  ;[1 1 1] Turn screen on
  (bind _aswbp_hud (Utilities|Casting|CastToWBP_HUD (Variables|/Game/FirstPerson/Blueprints/BP_FirstPersonCharacter.BP_FirstPersonCharacter_C|Gethud_Ref _playerrefmaster)))
  (bind _isvisible (Default|ToggleMonitorScreen _aswbp_hud))
  (if _isvisible
    (Variables|/Game/FirstPerson/Blueprints/BP_FirstPersonCharacter.BP_FirstPersonCharacter_C|SetisSitting (Variables|Default|GetplayerRefMaster) true)
    (return true)
    (else
      (return false))))

(fn StandPlayerUp
  (bind _playerrefmaster (Variables|Default|GetplayerRefMaster))
  ;[1 1 1] change cursor and input mode
  (bind _action_output (Default|UpdateCursor (Variables|Default|GetplayerRefMaster) false false false true))
  (Development|PrintString _action_output)
  (Default|ChangeCamera _playerrefmaster false "None")
  (bind _aswbp_hud (Utilities|Casting|CastToWBP_HUD (Variables|/Game/FirstPerson/Blueprints/BP_FirstPersonCharacter.BP_FirstPersonCharacter_C|Gethud_Ref _playerrefmaster)))
  (bind _isvisible (Default|ToggleMonitorScreen _aswbp_hud))
  (if _isvisible
    (Development|PrintString "motherfucking failed standing up" true true "(R=1.000000,G=0.000000,B=0.243276,A=1.000000)" 1e+01)
    (return false)
    (else
      ;[1 1 1] Update Control Scheme
      (Default|ChangeControlScheme (Variables|Default|GetplayerRefMaster) "/Game/FirstPerson/Input/IMC_Walking.IMC_Walking")
      (Development|PrintString "mofo stood up" true true "(R=0.000000,G=1.000000,B=0.007329,A=1.000000)" 1e+01)
      (return true))))

(fn GetCameratoPosition
  (bind _outactors (Actor|GetAllActorsOfClass "/Script/CinematicCamera.CineCameraActor"))
  (bind _array_element (Utilities|Array|ForEachLoopwithBreak _outactors :!label _label)
    (:LoopBody
      (if (Actor|ActorHasTag _array_element "FPV_SitDown")
        (goto _label Break)))
    (:Completed
      (Transformation|SetWorldTransform (Variables|/Script/Engine.Actor|GetRootComponent _array_element) (Transformation|GetWorldTransform (Variables|Default|GetMonitorCameraPosition)) false true))))

(fn OnRepInteractToggle
  (Development|PrintString "notify received")
  (if (Variables|Default|GetInteractToggle)
    (Development|PrintString "Hello")
    (else
      (Development|PrintString "Hello2")))
  (CallFunction|SitPlayerDown))

(fn GetInteractionWidgetRef
  (return (Variables|Default|GetWidget)))