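; Main game instance that holds pause and construction-mode state and relays menu, pause and construction changes to the first-person player character.
; Each function casts player character 0 to BP_FirstPersonCharacter and calls its widget or mode-switch functions.
; PauseGame toggles engine pause, then refreshes the pause widget.
; Leaving construction mode re-enables collision on the queued wall actors and clears that list.
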(fn PlayerUpdateMenuStatus
  ;[1 1 1] Tells player BP to figure out if we are in main menu or not
  (bind _asbp_first_person_character (Utilities|Casting|CastToBP_FirstPersonCharacter (Game|GetPlayerCharacter 0)))
  (Default|WidgetUpdateBeginPlay _asbp_first_person_character))

(fn PlayerUpdatePauseStatus
  ;[1 1 1] Tells player BP to update the pausing widget
  (bind _asbp_first_person_character (Utilities|Casting|CastToBP_FirstPersonCharacter (Game|GetPlayerCharacter 0)))
  (bind _ispausedwidget (Default|WidgetUpdatePause _asbp_first_person_character false false))
  (return _ispausedwidget))

(fn PauseGame
  ;[1 1 1] Pauses the game
  (if (Game|IsGamePaused)
    (bind _returnvalue (Game|SetGamePaused false))
    (CallFunction|PlayerUpdatePauseStatus)
    (Variables|Default|SetisInPause _returnvalue)
    (return _returnvalue)
    (else
      (bind _returnvalue_2 (Game|SetGamePaused true))
      (CallFunction|PlayerUpdatePauseStatus)
      (Variables|Default|SetisInPause _returnvalue_2)
      (return _returnvalue_2))))

(fn PlayerUpdateConstructionMenu
  ;[1 1 1] When player changes between regular and construction mode
  (bind _asbp_first_person_character (Utilities|Casting|CastToBP_FirstPersonCharacter (Game|GetPlayerCharacter 0)))
  (bind _isinconstructionmode (Default|ConstructionModeSwitch _asbp_first_person_character))
  (bind _output_get (Variables|Default|SetisInConstruction _isinconstructionmode))
  (if (not _output_get)
    ;[1 1 1] Collision of wall assets gets updated
    (for _array_element (Variables|Default|GetobjectsThatNeedRecollision)
      (Collision|SetActorEnableCollision _array_element true))
    (Utilities|Array|Clear (Variables|Default|GetobjectsThatNeedRecollision))))