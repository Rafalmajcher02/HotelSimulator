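; BP_AIRoomMaster is a manager actor that finds the rooms in the level and reports their occupancy through debug prints.
; On BeginPlay it gathers all BPC_Room actors, enables player input, prints each room's index and Occupied or Free state, and adds to ArrayOfRooms.
; Pressing K prints the display name of each room found at startup.
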(event EventBeginPlay
  (bind _outactors (Actor|GetAllActorsOfClass "/Game/Blueprints/Room/AI_Room/BPC_Room.BPC_Room_C"))
  (Input|EnableInput (Game|GetPlayerController 0))
  (for _array_element _outactors
    (if (Variables|BP_AIRoomMaster_C|GetisOccupied _array_element)
      (Variables|Default|SettempVar "Occupied")
      (else
        (Variables|Default|SettempVar "Free")))
    (Development|PrintString (Utilities|String|ToString(Text) (Utilities|Text|FormatText "Room {Index} is {OccupationStatus}" (Variables|BP_AIRoomMaster_C|GetRoomIndex _array_element) (Variables|Default|GettempVar))) true true "(R=0.000000,G=0.660000,B=1.000000,A=1.000000)" 1e+01)
    (Utilities|Array|Add (Variables|Default|GetarrayOfRooms) 0))
  (Development|PrintString "No More Rooms Detected"))

(event Input|KeyboardEvents|K
  (params (Key :type Key%20Structure))
  (:Pressed
    (for _array_element (stale EventBeginPlay _outactors)
      (Development|PrintString (Utilities|GetDisplayName _array_element) true true "(R=0.000000,G=0.660000,B=1.000000,A=1.000000)" 17.0))))

(fn ConstructionScript)