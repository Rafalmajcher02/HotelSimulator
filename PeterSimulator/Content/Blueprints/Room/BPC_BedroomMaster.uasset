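; BPC_BedroomMaster builds the list of preplaced bedrooms that AI can use in the level.
; Its CollectAllRooms custom event, used to avoid running before the bedrooms, passes a DoOnce so repeated calls collect only once.
; It gathers BPCC_Bedroom actors tagged UsableBedroom into an array slotted by each room's RoomIndex, with debug prints.
; The finished array is copied to the RoomMaster held by GI_MainGameInstance.
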(event Custom|CollectAllRooms
  (Utilities|FlowControl|DoOnce false ; Prevents every single room firing the event and only does it once. Will use reset in future when needing to fire the event again
    (:Completed
      (bind _outactors (Actor|GetAllActorsOfClass "/Game/Blueprints/Room/BPCC_Bedroom.BPCC_Bedroom_C"))
      (for _array_element _outactors
        (if (Actor|ActorHasTag _array_element "UsableBedroom")
          (Utilities|Array|SetArrayElem (Variables|Default|GetusableBedroomsForAI) (Variables|BPC_BedroomMaster_C|GetroomIndex _array_element) _array_element true)
          (Development|PrintString (Utilities|String|ToString(Text) (Utilities|Text|FormatText "Room {name} with index {index} was added to general array" (Utilities|GetDisplayName _array_element) (Variables|BPC_BedroomMaster_C|GetroomIndex _array_element))) true true "(R=0.066792,G=0.115909,B=1.000000,A=1.000000)" 1e+01)))
      (Development|PrintString "BedroomMaster collected all AI bedrooms (preplaced in level by dev)" true true "(R=0.000000,G=1.000000,B=0.220168,A=1.000000)")
      (bind _asgi_main_game_instance (Utilities|Casting|CastToGI_MainGameInstance (Game|GetGameInstance)))
      (Variables|/Game/Blueprints/Room/BP_RoomMaster.BP_RoomMaster_C|SetusableBedroomsForAI (Variables|/Game/Blueprints/GameInstance/GI_MainGameInstance.GI_MainGameInstance_C|GetRoomMaster _asgi_main_game_instance) (Variables|Default|GetusableBedroomsForAI)))))

(fn ConstructionScript
  (|CallParentFunction))