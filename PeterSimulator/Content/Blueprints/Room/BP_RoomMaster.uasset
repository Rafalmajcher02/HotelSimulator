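; BP_RoomMaster is a room manager Blueprint that holds a list of bedrooms usable by AI.
; On BeginPlay it registers itself as the RoomMaster on GI_MainGameInstance.
; A DebugRoomList event builds a string of each bedroom's name and index and prints it on screen, with valid and invalid entries formatted identically.
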(event Custom|DebugRoomList
  (for (_array_element _array_index) (Variables|Default|GetusableBedroomsForAI)
    (Utilities|IsValid _array_element
      (:Is%20Valid
        (Variables|Default|SettempDebugString (Utilities|String|Append (Variables|Default|GettempDebugString) (Utilities|GetDisplayName _array_element) (Utilities|String|ToString(Text) (Utilities|Text|FormatText "-with index {index} - " _array_index)))))
      (:Is%20Not%20Valid
        (Variables|Default|SettempDebugString (Utilities|String|Append (Variables|Default|GettempDebugString) (Utilities|GetDisplayName _array_element) (Utilities|String|ToString(Text) (Utilities|Text|FormatText "-with index {index} - " _array_index)))))))
  (Development|PrintString (Variables|Default|GettempDebugString) true true "(R=1.000000,G=0.883787,B=0.000000,A=1.000000)" 99.0 "ny5t5"))

(event EventBeginPlay
  (bind _asgi_main_game_instance (Utilities|Casting|CastToGI_MainGameInstance (Game|GetGameInstance)))
  (Variables|/Game/Blueprints/GameInstance/GI_MainGameInstance.GI_MainGameInstance_C|SetRoomMaster _asgi_main_game_instance self))

(fn ConstructionScript)