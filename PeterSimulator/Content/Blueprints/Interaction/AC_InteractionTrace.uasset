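; Actor component that detects the interaction area the player's camera is looking at and triggers interaction with it.
; Each tick it line-traces from the camera on the Visibility channel, toggling focus when the hit BP_InteractionArea changes or is lost.
; Interact input on a zero-duration area calls InteractOnServer, which sends an interface message to the area's parent actor.
; Timed interactions are not handled yet, and debug trace drawing and prints remain active.
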(event Custom|TryToInteract
  (params (In :type Boolean))
  (if In
    (if (Variables|Default|GetisTracingInteractionArea)
      (bind _output_get (Variables|Default|SetInteract%20Duration (Variables|/Game/Blueprints/Interaction/InteractionArea/BP_InteractionArea.BP_InteractionArea_C|GetInteractDuration (Variables|Default|GetFocusedInteractionArea))))
      (if (not (> _output_get 0.0))
        (CallFunction|InteractonServer (Variables|Default|GetFocusedInteractionArea))))))

(event Custom|InteractOnServer
  (params (InteractionArea :type BP%20Interaction%20Area%20Object%20Reference))
  (Class|BPIInteraction|InterfaceInteract(Message) (Actor|GetParentActor InteractionArea)))

(event EventBeginPlay)

(event EventTick
  (params (DeltaSeconds :type Float%20%28single-precision%29))
  (CallFunction|Trace))

(fn Trace
  (bind _returnvalue (Game|GetPlayerCameraManager 0))
  (bind _returnvalue_2 (Transformation|GetActorLocation _returnvalue))
  (bind (_outhit _returnvalue_3) (Collision|LineTraceByChannel _returnvalue_2 (+ _returnvalue_2 (* (Math|Vector|GetForwardVector (Transformation|GetActorRotation _returnvalue)) (Variables|Default|GetLengh))) "TraceTypeQuery1" false 0 "ForDuration"))
  (if _returnvalue_3
    ;[1 1 1] Is It Not The Same?
    (if (!= (Variables|Default|GetFocusedActor) (.HitActor (Collision|BreakHitResult _outhit)))
      (Variables|Default|SetFocusedActor (.HitActor (Collision|BreakHitResult _outhit)))
      (CallFunction|TraceInteractionArea (== (Utilities|GetClass (.HitActor (Collision|BreakHitResult _outhit))) "/Game/Blueprints/Interaction/InteractionArea/BP_InteractionArea.BP_InteractionArea_C"))
      (Development|PrintString "Traced Something" true true "(R=0.000000,G=1.000000,B=0.226714,A=1.000000)" 2.0 "12341234"))
    (else
      (Development|PrintString "Traced Nothing" true true "(R=1.000000,G=0.000000,B=0.022377,A=1.000000)" 2.0 "12341234")
      (CallFunction|TraceInteractionArea false))))

(fn TraceInteractionArea
  (params (Trace :type Boolean))
  (if Trace
    (if (Variables|Default|GetisTracingInteractionArea)
      (Default|ToggleFocus (Variables|Default|GetFocusedInteractionArea) false))
    (bind _asbp_interaction_area (Utilities|Casting|CastToBP_InteractionArea (Variables|Default|GetFocusedActor)))
    (bind _output_get (Variables|Default|SetFocusedInteractionArea _asbp_interaction_area))
    (Default|ToggleFocus _output_get true)
    (Variables|Default|SetisTracingInteractionArea true)
    (elif (Variables|Default|GetisTracingInteractionArea)
      (Variables|Default|SetisTracingInteractionArea false)
      (Default|ToggleFocus (Variables|Default|GetFocusedInteractionArea) false)
      (Variables|Default|SetFocusedActor 0)
      (Variables|Default|SetFocusedInteractionArea 0))))