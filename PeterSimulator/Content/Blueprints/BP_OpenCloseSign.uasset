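; An interactable open/close sign that swaps its cube's material between open and closed versions, starting on closed.
; The interact interface event calls InteractOnServer, which flips InteractToggle, and that variable's RepNotify applies the matching material.
; A focus event toggles custom depth rendering on the cube and prints the focus value as debug text.
; GetInteractionWidgetRef is an empty stub.
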(event Custom|InteractOnServer
  (Variables|Default|SetInteractToggle (not (Variables|Default|GetInteractToggle))))

(event Custom|CustomEvent
  (params (Focus :type Boolean))
  (Development|PrintString (Utilities|String|ToString(Boolean) Focus) true true "(R=1.000000,G=0.000000,B=0.148264,A=1.000000)" 5.0 "654365346")
  (Rendering|SetRenderCustomDepth (Variables|Default|GetCube) Focus))

(event EventBeginPlay
  (Rendering|Material|SetMaterial (Variables|Default|GetCube) 0 "/Game/Materials/MI_Close.MI_Close"))

(event EventInterfaceInteract
  (CallFunction|InteractonServer))

(fn ConstructionScript)

(fn OnRepInteractToggle
  (bind _cube (Variables|Default|GetCube))
  (if (Variables|Default|GetInteractToggle)
    (Rendering|Material|SetMaterial _cube 0 "/Game/Materials/MI_Open.MI_Open")
    (else
      (Rendering|Material|SetMaterial _cube 0 "/Game/Materials/MI_Close.MI_Close"))))

(fn GetInteractionWidgetRef
  (return 0))