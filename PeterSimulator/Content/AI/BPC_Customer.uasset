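; Interactable customer actor for reception, letting the player assign or deny a room to an AI guest.
; Focus highlights it via custom depth, while interaction flips InteractToggle, whose OnRep opens the room selection widget, stops the player and switches to UI input.
; Toggling off reads the player's AI command, writes denial or room index to the AI Blackboard, and, except on room selection, closes the menu.
; Includes extensive debug prints and a debug light.
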(event Custom|InteractOnServer
  ;[1 1 1] make sure to copy over bottom then top
  ;;[1 1 1] Set replicate correctly in details
  (Variables|Default|SetInteractToggle (not (Variables|Default|GetInteractToggle)))
  (Development|PrintString "toggled"))

(event Custom|UpdateRoomIndexEvent
  (bind _aic_ref (Variables|Default|Getaic_ref))
  (Class|BlackboardComponent|SetValueasInt (Variables|/Script/AIModule.AIController|GetBlackboard (Variables|Default|Getaic_ref)) (Variables|Default|GetRoomIndex) (Variables|Default|GetAssignedRoomIndex))
  (Development|PrintString (Utilities|String|ToString(Text) (Utilities|Text|FormatText "{ac} room index was set as {index} in {blackboard}" (Utilities|GetDisplayName _aic_ref) (Variables|Default|GetAssignedRoomIndex) (Utilities|GetDisplayName (Variables|/Script/AIModule.AIController|GetBlackboard _aic_ref)))) true true "(R=0.703719,G=1.000000,B=0.950004,A=1.000000)" 2.0 "5435346436"))

(event Custom|ForcedInteract
  ;[1 1 1] Custom part to override other bools
  ;[1 1 1] make sure to copy over bottom then top
  (CallFunction|InteractonServer))

(event EventBeginPlay
  (Utilities|IsValid (Variables|Default|Getaic_ref)
    (:Is%20Valid
      (Development|PrintString "AIC Ref VALID" true true "(R=0.000000,G=1.000000,B=0.238766,A=1.000000)" 11.0))
    (:Is%20Not%20Valid
      (Development|PrintString "AIC Ref inVALID" true true "(R=1.000000,G=0.000000,B=0.000000,A=1.000000)" 11.0))))

(event EventTick
  (params (DeltaSeconds :type Float%20%28single-precision%29))
  (Development|PrintString (Utilities|String|ToString(Text) (Utilities|Text|FormatText "My AI assinged room index is {index}" (Variables|Default|GetAssignedRoomIndex))) true true "(R=0.000000,G=0.104877,B=1.000000,A=1.000000)" 346346.0 "Non543534e"))

(event EventInterfaceToggleFocus
  (params (Focus :type Boolean))
  ;[1 1 1] When copying this make sure the bp has bpi_interface added and childactor added correctly
  ;;[1 1 1] Custom part for making something only sometimes interactable
  (if (Variables|Default|GetisInteractable)
    (Development|PrintString (Utilities|String|ToString(Boolean) Focus) true true "(R=1.000000,G=0.000000,B=0.148264,A=1.000000)" 5.0 "654365346")
    (Rendering|SetRenderCustomDepth (Variables|Default|GetCylinder) Focus)))

(event EventInterfaceInteract
  ;[1 1 1] make sure to copy over bottom then top
  (if (Variables|Default|GetisInteractable) ; Custom mod to make interaction toggleable
    (CallFunction|InteractonServer)))

(fn ConstructionScript)

(fn OnRepInteractToggle
  (bind _pointlight (Variables|Default|GetPointLight))
  ;[1 1 1] Doing it this way instead of BeginPlay helped getting references after they were ready in the player to begin with. Local because I don't believe I'll need them anywhere else at the moment.
  (bind _asbp_first_person_character (Utilities|Casting|CastToBP_FirstPersonCharacter (Game|GetPlayerCharacter 0)))
  (LocalVariables|SetplayerRefLocal _asbp_first_person_character)
  (LocalVariables|SetHUD_RefLocal (Variables|/Game/FirstPerson/Blueprints/BP_FirstPersonCharacter.BP_FirstPersonCharacter_C|Gethud_Ref _asbp_first_person_character))
  ;[1 1 1] Just debug
  (Development|PrintString "notify received")
  (if (Variables|Default|GetInteractToggle)
    ;[1 1 1] This is debugging light that turns on on interacted actors. Helps understanding if interaction happened in dev stages. Remove this when releasing product
    (Rendering|SetVisibility _pointlight true false)
    ;[1 1 1] Validity Checks
    (Utilities|IsValid (LocalVariables|GetHUD_RefLocal)
      (:Is%20Valid
        (Utilities|IsValid (Variables|Default|GetRoomSelectionScreenWidget)
          (:Is%20Valid
            _)
          (:Is%20Not%20Valid
            ;[1 1 1] Creates the widget
            (bind _returnvalue (UserInterface|CreateWidget "/Game/UserInterface/Menues/WBP_CustomerRoomSelectionMenu.WBP_CustomerRoomSelectionMenu_C" (Game|GetPlayerController 0)))
            (Variables|Default|SetRoomSelectionScreenWidget _returnvalue)))
        (UserInterface|Viewport|AddtoViewport (Variables|Default|GetRoomSelectionScreenWidget) 0)
        ;[1 1 1] Prevents player from retaining velocity if interacted with customer while walking. Important to allow the cancel button to function and for player to not wonder off into sunset when selecting rooms
        (Components|Movement|StopMovementImmediately (Variables|/Script/Engine.Character|GetCharacterMovement (LocalVariables|GetplayerRefLocal)))
        (Default|ManualMovementStopEvent (LocalVariables|GetplayerRefLocal))
        (bind _currentcursorstatus (Default|UpdateCursor (LocalVariables|GetplayerRefLocal) false false true false))
        ;[1 1 1] Debug
        (if _currentcursorstatus
          (Development|PrintString "CURSOR ON via customer reception" true true "(R=1.000000,G=0.000000,B=0.217000,A=1.000000)" 5.0 "Rec325")
          (else
            (Development|PrintString "CURSOR FAILED ON via customer reception" true true "(R=1.000000,G=0.000000,B=0.217000,A=1.000000)" 5.0 "Rec325"))))
      (:Is%20Not%20Valid
        (Development|PrintString "HUD REF INVALID in BP_Customer when accessing Player's room menu on interaction at reception" true true "(R=1.000000,G=0.000000,B=0.217000,A=1.000000)" 5.0 "Rec325")))
    (else
      ;[1 1 1] New AI Command
      (switch string (Variables|/Game/FirstPerson/Blueprints/BP_FirstPersonCharacter.BP_FirstPersonCharacter_C|GetAI_Command (LocalVariables|GetplayerRefLocal))
        (:Default
          (Development|PrintString "AI Command None")
          (Rendering|SetVisibility _pointlight false false :!label _label)
          (Utilities|IsValid (LocalVariables|GetHUD_RefLocal)
            (:Is%20Valid
              (Utilities|IsValid (Variables|Default|GetRoomSelectionScreenWidget)
                (:Is%20Valid
                  ;[1 1 1] Removes the widget
                  (Widget|RemovefromParent (Variables|Default|GetRoomSelectionScreenWidget))
                  (Variables|Default|SetRoomSelectionScreenWidget 0))
                (:Is%20Not%20Valid
                  _))
              ;[1 1 1] Change back to gaming input scheme and cursor
              (Default|UpdateCursor (LocalVariables|GetplayerRefLocal) false false false true)
              ;[1 1 1] Debug
              (if true
                (Development|PrintString "CURSOR FAILED OFF via customer reception" true true "(R=1.000000,G=0.000000,B=0.217000,A=1.000000)" 5.0 "Rec325")
                (else
                  (Development|PrintString "CURSOR OFF via customer reception" true true "(R=1.000000,G=0.000000,B=0.217000,A=1.000000)" 5.0 "Rec325"))))
            (:Is%20Not%20Valid
              (Development|PrintString "HUD REF INVALID in BP_Customer when accessing Player's room menu on interaction at reception" true true "(R=1.000000,G=0.000000,B=0.217000,A=1.000000)" 5.0 "Rec325"))))
        (:Off
          (Development|PrintString "AI Command Off")
          (goto _label))
        (:DenyRoom
          ;[1 1 1] Sets BB variable to tell BT room was denied.
          (AI|Components|Blackboard|SetValueasBool (Variables|/Script/AIModule.AIController|GetBlackboard (Variables|Default|Getaic_ref)) (Variables|Default|GetisDeniedService) true)
          (Development|PrintString "AI Command DeniedRoom")
          (goto _label))
        (:RoomSelect
          (Class|BlackboardComponent|SetValueasInt (Variables|/Script/AIModule.AIController|GetBlackboard (Variables|Default|Getaic_ref)) (Variables|Default|GetRoomIndex))
          (Development|PrintString "AI Command. Room Selected"))))))

(fn ToggleInteractibility
  ;[1 1 1] Simple flip the active child responsible for interactability of the main actor
  (if (Variables|Default|GetisInteractable)
    (Variables|Default|SetisInteractable false)
    (return false)
    (else
      (Variables|Default|SetisInteractable true)
      (return true))))

(fn GenerateRandomText
  (params (PositiveMessage? :type Boolean))
  (if (not PositiveMessage?)
    (Rendering|Components|TextRender|SetText (Variables|Default|GetRandom%20Message%20Text) (Utilities|Text|ToText(String) (Utilities|Array|Get(acopy) (LocalVariables|GetrandomNegativeMessages) (Math|Random|RandomInteger 5))))
    (return)))

(fn GetInteractionWidgetRef
  (return (Variables|Default|GetWidget)))